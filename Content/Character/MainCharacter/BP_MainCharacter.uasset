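; Player character with world-axis Enhanced Input movement, switchable melee and ranged attack modes, and a gold counter.
; Melee jumps the animation state machine to Attack, and NotifyAttack applies damage through BPC_Salud on actors overlapping CollisionAttack.
; Ranged mode shows the cursor and spawns BP_Proyectil at the actor's transform.
; Before spawning, Disparar feeds the cursor look-at yaw into SetActorLocation's Z rather than a rotation.
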(event Input|EnhancedActionEvents|EnhancedInputActionIA_Melee
  (params (ActionValue :type Boolean) (ElapsedSeconds :type Float%20%28double-precision%29) (TriggeredSeconds :type Float%20%28double-precision%29) (InputAction :type Input%20Action%20Object%20Reference :default "/Game/Character/MainCharacter/Input/Actions/IA_Melee.IA_Melee"))
  (Variables|Default|SetE%20state "NewEnumerator1")
  (Development|PrintString "Estoy modo melee" true true "(R=0.687500,G=0.000000,B=0.034889,A=1.000000)")
  (Variables|/Script/Engine.PlayerController|SetbShowMouseCursor (Game|GetPlayerController 0) false))

(event Input|EnhancedActionEvents|EnhancedInputActionIA_Rango
  (params (ActionValue :type Boolean) (ElapsedSeconds :type Float%20%28double-precision%29) (TriggeredSeconds :type Float%20%28double-precision%29) (InputAction :type Input%20Action%20Object%20Reference :default "/Game/Character/MainCharacter/Input/Actions/IA_Rango.IA_Rango"))
  (Variables|Default|SetE%20state "NewEnumerator2")
  (Development|PrintString "Estoy modo Rango" true true "(R=0.085210,G=1.000000,B=0.000000,A=1.000000)")
  (Variables|/Script/Engine.PlayerController|SetbShowMouseCursor (Game|GetPlayerController 0) true))

(event Input|EnhancedActionEvents|EnhancedInputActionIA_Move
  (params (ActionValue :type Vector%202D%20Structure) (ElapsedSeconds :type Float%20%28double-precision%29) (TriggeredSeconds :type Float%20%28double-precision%29) (InputAction :type Input%20Action%20Object%20Reference :default "/Game/Character/MainCharacter/Input/Actions/IA_Move.IA_Move"))
  (Pawn|Input|AddMovementInput "1.000000,0.000000,0.000000" (.x ActionValue) false)
  (Pawn|Input|AddMovementInput "0.000000,1.000000,0.000000" (.y ActionValue) false))

(event Input|EnhancedActionEvents|EnhancedInputActionIA_Ataque
  (params (ActionValue :type Boolean) (ElapsedSeconds :type Float%20%28double-precision%29) (TriggeredSeconds :type Float%20%28double-precision%29) (InputAction :type Input%20Action%20Object%20Reference :default "/Game/Character/MainCharacter/Input/Actions/IA_Ataque.IA_Ataque"))
  (:Started
    (switch Utilities|FlowControl|Switch|SwitchonE_State (Variables|Default|GetState)
      (:NewEnumerator1
        (if (not (Utilities|Enum|Equal(Enum) (Utilities|GetDisplayName (Class|PaperZDAnimPlayer|GetCurrentAnimSequence (Class|PaperZDAnimInstance|GetPlayer (Variables|Default|GetAnimInstance)))) "Attack"))
          (Class|PaperZDAnimInstance|JumptoNode (Variables|Default|GetAnimInstance) "Attack" "None")))
      (:NewEnumerator2
        (CallFunction|Disparar)))))

(event EventBeginPlay
  (|CallParentFunction)
  (bind _asplayer_controller (Utilities|Casting|CastToPlayerController (Pawn|GetController)))
  (Input|AddMappingContext (PlayerController|LocalPlayerSubsystems|GetEnhancedInputLocalPlayerSubsystem _asplayer_controller) "/Game/Character/MainCharacter/Input/IMC_Default.IMC_Default" 0 "(bIgnoreAllPressedKeysUntilRelease=True,bForceImmediately=False,bNotifyUserSettings=False)")
  (Development|ExecuteConsoleCommand "Show Collision" 0))

(event EventSumarOro
  (params (Orito :type Integer))
  (CallFunction|AddOro Orito))

(event EventNotifyAttack
  (for _array_element (Collision|GetOverlappingActors (Variables|Default|GetCollisionAttack) 0 :!class /Script/Engine.PrimitiveComponent)
    (Default|AplicarDaño (Actor|GetComponentbyClass _array_element "/Game/Character/MainCharacter/Componentes/BPC_Salud.BPC_Salud_C") (Variables|Default|GetDaño))))

(fn ConstructionScript
  (|CallParentFunction))

(fn AddOro
  (params (OroEntrante :type Integer))
  (bind _output_get (Variables|Default|SetOro (+ OroEntrante (Variables|Default|GetOro))))
  (Development|PrintString (Utilities|String|Append "Tu oro es: 
" (Utilities|String|ToString(Integer) _output_get))))

(fn Disparar
  (Transformation|SetActorLocation (Math|Vector|MakeVector 0.0 0.0 (.yaw (Math|Rotator|FindLookatRotation (Math|Vector|MakeVector 0.0 0.0 0.0) (- (.ImpactPoint (Collision|BreakHitResult (.HitResult (Game|Player|GetHitResultUnderCursorbyChannel (Game|GetPlayerController 0) "TraceTypeQuery1" true)))) (Transformation|GetActorLocation))))) false false)
  (Game|SpawnActorfromClass "/Game/Objects/Proyectil/BP_Proyectil.BP_Proyectil_C" (Transformation|GetActorTransform) "Undefined" "MultiplyWithRoot" 0 0))