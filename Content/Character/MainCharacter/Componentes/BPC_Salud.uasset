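; BPC_Salud is a health component for the main character that tracks current and maximum life.
; AplicarDaño subtracts damage and clamps life between zero and the maximum.
; It then fires the SeDestruyo dispatcher when life reaches zero, or SeHaRealizadoDaño otherwise, printing a debug message in each case.
; The event graph holds only disabled BeginPlay and Tick stubs.
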(event EventBeginPlay)

(event EventTick
  (params (DeltaSeconds :type Float%20%28single-precision%29)))

(fn AplicarDaño
  (params (Daño :type Float%20%28double-precision%29))
  (bind _output_get (Variables|Default|SetVidaActual (Math|Float|Clamp(Float) (- (Variables|Default|GetVidaActual) Daño) 0.0 (Variables|Default|GetVidaMáxima))))
  (if (== _output_get 0.0)
    (Development|PrintString "moriste")
    (Default|CallSeDestruyo)
    (else
      (Development|PrintString "Se quito vida")
      (Default|CallSeHaRealizadoDaño))))