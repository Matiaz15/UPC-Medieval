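; Enemy character Blueprint that handles death with a gold drop and receives targets for its AI.
; When the BPCSalud health component signals destruction, it starts a death animation override, waits briefly, spawns BP_Oro_1 at its transform and destroys itself.
; SetearObjetivo writes the target to the controller's Blackboard and prints a debug message.
; AtaqueBase only defers to its parent, and the Disparo (shot) event is an empty stub.
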(event Custom|Destruirse
  (|PlayAnimationOverridewithCallbacks (Variables|/Script/PaperZD.PaperZDAnimationComponent|GetAnimInstance (Variables|Default|GetAnimationComponent)) (Variables|Default|GetAnimacion%20muerte) "Attack" 1.0 0.0
    (:then
      (Utilities|FlowControl|Delay 0.5)
      (Game|SpawnActorfromClass "/Game/Objects/BP_Oro_1.BP_Oro_1_C" (Transformation|GetActorTransform) "Undefined" "MultiplyWithRoot" 0 0)
      (Actor|DestroyActor))))

(event EventBeginPlay
  (|CallParentFunction)
  (EventDispatchers|BindEventtoSeDestruyo (Variables|Default|GetBPC_Salud) (delegate Custom|Destruirse)))

(event EventDisparo
  (params (ObjetivoPosición :type Vector :default "0, 0, 0")))

(event EventSetearObjetivo
  (params (Objetivo :type Actor%20Object%20Reference))
  (AI|Components|Blackboard|SetValueasObject (AI|GetBlackboard (Pawn|GetController)) (Variables|Default|GetObjetivoBBKeyName) Objetivo)
  (Development|PrintString "Se seteo objetivo"))

(fn ConstructionScript
  (|CallParentFunction))

(fn AtaqueBase
  (params (Animacion%20de%20ataque :type Paper%20ZD%20Anim%20Sequence%20Object%20Reference))
  (|CallParentFunction Animacion%20de%20ataque))