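; BP_Skeleton is a skeleton enemy character that handles its own death and receives an AI target.
; On BeginPlay it binds to the BPCSalud health component's SeDestruyo event, which destroys the actor after a short delay.
; SetearObjetivo writes the given target into the controller's Blackboard under the ObjetivoBBKeyName key and prints a debug message.
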(event Custom|Destruirse
  (Utilities|FlowControl|Delay 0.2)
  (Actor|DestroyActor))

(event EventBeginPlay
  (|CallParentFunction)
  (EventDispatchers|BindEventtoSeDestruyo (Variables|Default|GetBPC_Salud) (delegate Custom|Destruirse)))

(event EventSetearObjetivo
  (params (Objetivo :type Actor%20Object%20Reference))
  (AI|Components|Blackboard|SetValueasObject (AI|GetBlackboard (Pawn|GetController)) (Variables|Default|GetObjetivoBBKeyName) Objetivo)
  (Development|PrintString "Se seteo objetivo"))

(fn ConstructionScript
  (|CallParentFunction))