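; BP_CharacterBase is a base character Blueprint with health-damage notification and a basic attack.
; On BeginPlay it binds UpdateUI to the BPCSalud component's damage event, currently only printing a debug string.
; AtaqueBase plays a PaperZD animation override in the Attack slot, gated by Atacando, which both start and completion set true, so it never resets here.
; The Ataque function and construction script are empty.
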(event Custom|Update%20UI
  (Development|PrintString "dasdsad"))

(event Custom|AtaqueBase
  (if (not (Variables|Default|GetbAtacando?))
    (|PlayAnimationOverridewithCallbacks (Variables|/Script/PaperZD.PaperZDAnimationComponent|GetAnimInstance (Variables|Default|GetAnimationComponent)) (Variables|Default|GetAnimación%20de%20Ataque) "Attack" 1.0 0.0
      (:then
        (Variables|Default|SetbAtacando? true))
      (:OnCompleted
        (Variables|Default|SetbAtacando? true)))))

(event EventBeginPlay
  (EventDispatchers|BindEventtoSeHaRealizadoDaño (Variables|Default|GetBPC_Salud) (delegate Custom|Update%20UI)))

(fn ConstructionScript)

(fn Ataque)