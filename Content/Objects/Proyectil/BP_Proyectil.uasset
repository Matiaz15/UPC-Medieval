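; BP_Proyectil is a projectile actor that deals damage to what it hits.
; On BeginPlay it launches its ProjectileMovement along Direction at Speed and sets a short life span.
; On any actor overlap it applies Daño through the other actor's BPC_Salud health component when present, then destroys itself either way.
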(event EventBeginPlay
  (bind _projectilemovement (Variables|Components|GetProjectileMovement))
  (bind _output_get (Variables|/Script/Engine.ProjectileMovementComponent|SetInitialSpeed _projectilemovement (Variables|Default|GetSpeed)))
  (bind _output_get_2 (Variables|/Script/Engine.ProjectileMovementComponent|SetMaxSpeed _projectilemovement _output_get))
  (Variables|/Script/Engine.MovementComponent|SetVelocity _projectilemovement (* _output_get_2 (Variables|Default|GetDirection)))
  (Actor|SetLifeSpan 3.0))

(event Collision|EventActorBeginOverlap
  (params (OtherActor :type Actor%20Object%20Reference))
  (bind _returnvalue (Actor|GetComponentbyClass OtherActor "/Game/Character/MainCharacter/Componentes/BPC_Salud.BPC_Salud_C"))
  (Utilities|IsValid _returnvalue
    (:Is%20Valid
      (Default|AplicarDaño _returnvalue (Variables|Default|GetDaño))
      (Actor|DestroyActor))
    (:Is%20Not%20Valid
      (Actor|DestroyActor))))

(fn ConstructionScript)